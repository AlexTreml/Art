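; BP_Camera_Track is a track-bound camera actor that makes itself the player's view target on BeginPlay.
; If LookActor is already valid, SortReference replaces it with the player's BP_ThirdPersonCharacter.
; FMoveCamera snaps CameraArm to the point on CameraTrack closest to LookActor's location, offset back by FollowDistance along world X.
; The move runs only once at BeginPlay, since Tick is disabled.
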(event Custom|SortReference
  (Utilities|IsValid (Variables|Default|GetLookActor)
    (:Is%20Valid
      (bind _asbp_third_person_character (Utilities|Casting|CastToBP_ThirdPersonCharacter (Game|GetPlayerCharacter 0)))
      (Variables|Default|SetLookActor _asbp_third_person_character))))

(event Custom|SetCamera
  (Game|Player|SetViewTargetwithBlend (Game|GetPlayerController 0) self 0.0 "VTBlend_Linear" 0.0 false))

(event EventBeginPlay
  (CallFunction|SortReference)
  (CallFunction|SetCamera)
  (CallFunction|FMoveCamera))

(event Collision|EventActorBeginOverlap
  (params (OtherActor :type Actor%20Object%20Reference)))

(event EventTick
  (params (DeltaSeconds :type Float%20%28single-precision%29)))

(fn ConstructionScript)

(fn FMoveCamera
  (Utilities|IsValid (Variables|Default|GetLookActor)
    (:Is%20Valid
      (Transformation|SetWorldLocation (Variables|Default|GetCameraArm) (Spline|FindLocationClosesttoWorldLocation (Variables|Default|GetCameraTrack) (- (Transformation|GetActorLocation (Variables|Default|GetLookActor)) (Math|Vector|MakeVector (Variables|Default|GetFollowDistance) 0.0 0.0)) "World") false false))))