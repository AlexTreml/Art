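; PlayerProjectile is an actor for a projectile that explodes when its trigger overlaps anything other than the player character.
; On overlap, a helper spawns an explosion emitter at the trigger location and plays a 2D sound, then the projectile destroys itself.
; Overlapped actors tagged "Destroy" are also destroyed, and a macro filters out the player.
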(event OnComponentBeginOverlap(ProjectileExplosionTrigger)
  (params (OverlappedComponent :type Primitive%20Component%20Object%20Reference) (OtherActor :type Actor%20Object%20Reference) (OtherComp :type Primitive%20Component%20Object%20Reference) (OtherBodyIndex :type Integer) (bFromSweep :type Boolean) (SweepResult :type Hit%20Result%20Structure%20%28by%20ref%29))
  ;[1 1 1] On projectile trigger spawn vfx and sfx, then destory
  (Utilities|PlayerOverlaps OtherActor
    (:false
      (if (Actor|ActorHasTag OtherActor "Destroy")
        (CallFunction|SpawnVFXandSound "/Game/StarterContent/Particles/P_Explosion.P_Explosion" "/Game/StarterContent/Audio/Explosion01.Explosion01")
        (Actor|DestroyActor OtherActor)
        (Actor|DestroyActor)
        (else
          (CallFunction|SpawnVFXandSound "/Game/StarterContent/Particles/P_Explosion.P_Explosion" "/Game/StarterContent/Audio/Explosion01.Explosion01")
          (Actor|DestroyActor))))))

(event Custom|DestroyTagObjects
  ;[1 1 1] On projectile trigger spawn vfx and sfx, then destory
  (Utilities|IsValid (stale OnComponentBeginOverlap(ProjectileExplosionTrigger) OtherActor)
    (:Is%20Valid
      (Actor|DestroyActor (stale OnComponentBeginOverlap(ProjectileExplosionTrigger) OtherActor)))))

(event EventBeginPlay)

(event Collision|EventActorBeginOverlap
  (params (OtherActor :type Actor%20Object%20Reference)))

(event EventTick
  (params (DeltaSeconds :type Float%20%28single-precision%29)))

(fn ConstructionScript)

(fn SpawnVFXandSound
  (params (SpawnVFX :type Particle%20System%20Object%20Reference) (Spawn%20SFX :type Sound%20Base%20Object%20Reference))
  (Effects|SpawnEmitteratLocation SpawnVFX (Transformation|GetWorldLocation (Variables|Default|GetProjectileExplosionTrigger)))
  (Audio|PlaySound2D Spawn%20SFX 1.0 1.0 0.0 0 0))