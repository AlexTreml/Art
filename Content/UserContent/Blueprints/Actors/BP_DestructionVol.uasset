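; Box trigger volume that changes the player character's health over time, as damage or healing, while an overlap lasts.
; Begin overlap starts a fast looping timer that passes DamageHealth through SetHealthMessage, then reads health back with GetHealthMessage.
; The timer stops on end overlap or when health reaches either limit of the 0–100 range.
; PlayerOverlaps compares the actor to the player but returns no result, so it does not visibly filter overlaps.
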(event OnComponentBeginOverlap(Box)
  (params (OverlappedComponent :type Primitive%20Component%20Object%20Reference) (OtherActor :type Actor%20Object%20Reference) (OtherComp :type Primitive%20Component%20Object%20Reference) (OtherBodyIndex :type Integer) (bFromSweep :type Boolean) (SweepResult :type Hit%20Result%20Structure%20%28by%20ref%29))
  ;[1 1 1] Setting health if >= to 100 or <+ 0 stopping timer (so health will stop incrementing at 100 and damage stop at 0) and timer will stop
  ;;[1 1 1] Comment
  (CallFunction|PlayerOverlaps OtherActor)
  (bind _returnvalue (Utilities|Time|SetTimerbyEvent (delegate Custom|DamageOverTime) 0.02 true)))

(event OnComponentEndOverlap(Box)
  (params (OverlappedComponent :type Primitive%20Component%20Object%20Reference) (OtherActor :type Actor%20Object%20Reference) (OtherComp :type Primitive%20Component%20Object%20Reference) (OtherBodyIndex :type Integer))
  ;[1 1 1] At end of overlap stop the damage/heal timer
  (CallFunction|PlayerOverlaps OtherActor)
  (CallFunction|StopDamage/HealTimer))

(event Custom|DamageOverTime
  (bind _returnvalue (Game|GetPlayerCharacter 0))
  ;[1 1 1] Setting health if >= to 100 or <+ 0 stopping timer (so health will stop incrementing at 100 and damage stop at 0) and timer will stop
  ;;[1 1 1] Comment
  (Class|PlayerInterface|SetHealth(Message) _returnvalue (Variables|Damage/Heal|GetDamageHealth))
  (bind _health (Class|PlayerInterface|GetHealth(Message) _returnvalue))
  (if (or (<= _health 0.0) (>= _health 1e+02))
    (CallFunction|StopDamage/HealTimer)))

(event Custom|StopDamage/HealTimer
  ;[1 1 1] Setting health if >= to 100 or <+ 0 stopping timer (so health will stop incrementing at 100 and damage stop at 0) and timer will stop
  ;;[1 1 1] Comment
  (Utilities|Time|ClearandInvalidateTimerbyHandle (stale OnComponentBeginOverlap(Box) _returnvalue))
  (Development|PrintString "TimerisStopped"))

(event EventBeginPlay)

(event Collision|EventActorBeginOverlap
  (params (OtherActor :type Actor%20Object%20Reference)))

(event EventTick
  (params (DeltaSeconds :type Float%20%28single-precision%29)))

(fn ConstructionScript)

(fn PlayerOverlaps
  (params (Player :type Object%20Object%20Reference))
  (if (== Player (Game|GetPlayerCharacter 0))
    (return)))